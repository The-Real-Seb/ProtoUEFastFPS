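; Actor component for the FPS player character that turns movement speed into a damage bonus and a speed-driven camera FOV.
; GetBonusDamage scales owner velocity magnitude linearly above a base of one.
; Tick prints that value and smoothly widens or narrows the FOV from it.
; GetBonusBulletSpeed scales only the world X of the unit direction opposite the given velocity, so it ignores magnitude.
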(event `self.ReceiveBeginPlay`
  (bind _asbp_fpsplayer_character (cast `/Game/Proto/BP/BP_FPSPlayerCharacter` (`self.GetOwner`)))
  (set `self.owner` _asbp_fpsplayer_character))

(event `self.ReceiveTick`
  (params (DeltaSeconds :type "Float (single-precision)"))
  (bind _camera (`/Game/Proto/BP/BP_FPSPlayerCharacter.Camera` (`self.owner`)))
  (bind _damagemultiply (`self.Get Bonus Damage`))
  (`KismetSystemLibrary.PrintString` (`KismetStringLibrary.Conv_DoubleToString` _damagemultiply) true true (struct :`G` 0.66 :`B` 1.0 :`A` 1.0) 0.0)
  (`CameraComponent.SetFieldOfView` _camera (`KismetMathLibrary.Lerp` (`CameraComponent.FieldOfView` _camera) (`KismetMathLibrary.Lerp` 95.0 160.0 (`KismetMathLibrary.NormalizeToRange` _damagemultiply 0.0 12.0)) (* DeltaSeconds 25.0))))

(fn `Get Bonus Damage`
  (returns (damageMultiply :type "Float (double-precision)"))
  (return (+ (* (`self.bonusMultiply`) (/ (`KismetMathLibrary.VSize` (`Actor.GetVelocity` (`self.owner`))) 1000.0)) 1.0)))

(fn `GetBonusBulletSpeed`
  (params (velocity :type "Vector Structure"))
  (returns (bulletSpeed :type "Float (double-precision)"))
  (bind _returnvalue_x (`KismetMathLibrary.BreakVector` (`KismetMathLibrary.GetDirectionUnitVector` velocity)))
  (return (* (`self.speedMultiply`) _returnvalue_x)))