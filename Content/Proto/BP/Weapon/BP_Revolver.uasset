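; BP_Revolver is a prototype hitscan revolver, a child weapon whose Prepare, Shoot and OnShoot only call the parent.
; Fire runs a Visibility line trace from the owning BP_CharacterBase's LineOriginPoint along its forward vector out to FireRange, with timed debug drawing.
; A hit BP_EnemyBase takes Damage through its health component's OnHit; other hits are ignored.
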(event `self.Prepare`
  (`parent.Prepare`))

(event `self.Shoot`
  (`parent.Shoot`))

(fn `Fire`
  (bind _ascharacter (cast `Character` (`self.GetOwner`)))
  (bind _asbp_character_base (cast `/Game/Proto/BP/BP_CharacterBase` (`Controller.K2_GetPawn` (`Pawn.GetController` _ascharacter))))
  (bind _lineoriginpoint (`/Game/Proto/BP/BP_CharacterBase.LineOriginPoint` _asbp_character_base))
  (bind _returnvalue (`SceneComponent.K2_GetComponentLocation` _lineoriginpoint))
  (bind _outhit (`KismetSystemLibrary.LineTraceSingle` :`Start` _returnvalue :`End` (+ _returnvalue (* (`SceneComponent.GetForwardVector` _lineoriginpoint) (`self.FireRange`))) :`TraceChannel` "TraceTypeQuery1" :`DrawDebugType` "ForDuration"))
  (bind _asbp_enemy_base (cast `/Game/Proto/BP/Enemies/BP_EnemyBase` (`.HitActor` (`GameplayStatics.BreakHitResult` _outhit))))
  (`/Game/Proto/BP/BP_HealthComponent.onHit` (`/Game/Proto/BP/BP_CharacterBase.BP_HealthComponent` _asbp_enemy_base) (`self.Damage`)))

(fn `NewFunction_0`)

(fn `OnShoot`
  (`parent.OnShoot`))

(fn `UserConstructionScript`
  (`parent.UserConstructionScript`))