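; Laser gun weapon for the FPS player that locks a Niagara beam onto an enemy hit by the camera trace.
; While locked, Tick moves the beam end to the enemy and applies delayed damage.
; A re-armed timer raises the scale level, increasing damage and beam size.
; The lock breaks on release, a static-mesh obstruction, excessive aim deviation, target loss or OnHit returning true, without restoring Damage.
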(event `self.ReceiveTick`
  (params (DeltaSeconds :type "Float (single-precision)"))
  (bind _lazerbeam (`self.LazerBeam`))
  (bind _player (`self.Player`))
  (if (`self.bIsLockToTarget`)
    (`self.SetEnemyBeamEnd`)
    (`self.CheckBeamVision`)
    (`KismetSystemLibrary.Delay` 0.1)
    (`self.Apply Damage`)
    (else
      (`/Engine/EditorBlueprintResources/StandardMacros.IsValid` _lazerbeam
        (:`Is Valid`
          (`NiagaraComponent.SetVariableVec3` _lazerbeam "User.BeamEnd" (+ (`self.K2_GetActorLocation` _player) (* (`SceneComponent.GetForwardVector` (`/Game/Proto/BP/BP_FPSPlayerCharacter.Camera` _player)) (`self.FireRange`)))))))))

(event `self.ReceiveBeginPlay`
  (`self.GetPlayerController`))

(event `PrepareScale`
  (`KismetSystemLibrary.K2_SetTimerDelegate` (delegate `ScaleDamage`) (`self.ScaleDamageTime`)))

(event `ScaleDamage`
  (if (`self.bIsLockToTarget`)
    (`/Engine/EditorBlueprintResources/StandardMacros.IncrementInt` (`self.ScaleLevel`)
      (:`  `
        (set `self.ScaleDamageTime` (+ (`self.ScaleDamageTime`) (`|GetArrayItem` (`self.ScaleDamageTimer`) (`self.ScaleLevel`))))
        (`NiagaraComponent.SetNiagaraVariableInt` (`self.LazerBeam`) "User.BeamSize" (* (`self.ScaleLevel`) 40))
        (set `self.Damage` (`KismetMathLibrary.Conv_IntToDouble` (+ (`self.Damage`) (`|GetArrayItem` (`self.ScaleBonusDamage`) (`self.ScaleLevel`)))))
        (`self.PrepareScale`)))))

(fn `Apply Damage`
  (bind _enemylock (`self.EnemyLock`))
  (`/Engine/EditorBlueprintResources/StandardMacros.IsValid` _enemylock
    (:`Is Valid`
      (bind _bisdead (`/Game/Proto/BP/BP_HealthComponent.onHit` (`/Game/Proto/BP/Enemies/BP_EnemyBase.BP_HealthComponent` _enemylock) (`self.Damage`) false 0.0))
      (if _bisdead
        (`self.OnReleaseShoot`))
      (`/Game/Proto/BP/BP_FPSPlayerCharacter.HitMarker` (`self.Player`)))))

(fn `CastEnemyLock`
  (returns (OutHit :type "HitResult Structure"))
  (`/Engine/EditorBlueprintResources/StandardMacros.IsValid` (`self.EnemyLock`)
    (:`Is Valid`
      (bind _outhit (`KismetSystemLibrary.LineTraceSingle` (`SceneComponent.K2_GetComponentLocation` (`/Game/Proto/BP/BP_FPSPlayerCharacter.Camera` (`self.Player`))) (`self.K2_GetActorLocation` (`self.EnemyLock`)) "TraceTypeQuery3"))
      (return _outhit))))

(fn `CastLine`
  (returns (OutHit :type "HitResult Structure"))
  (bind _camera (`/Game/Proto/BP/BP_FPSPlayerCharacter.Camera` (`self.Player`)))
  (bind _returnvalue (`SceneComponent.K2_GetComponentLocation` _camera))
  (bind _outhit (`KismetSystemLibrary.LineTraceSingle` _returnvalue (+ _returnvalue (* (`SceneComponent.GetForwardVector` _camera) (`self.FireRange`))) "TraceTypeQuery3"))
  (return _outhit))

(fn `CheckBeamVision`
  (if (and true (`self.CheckLostFocusBeam`) (`KismetSystemLibrary.IsValid` (`self.EnemyLock`)))
    (`self.OnReleaseShoot`)))

(fn `CheckLostFocusBeam`
  (returns (ReturnValue :type Boolean))
  (bind _enemylock (`self.EnemyLock`))
  (`/Engine/EditorBlueprintResources/StandardMacros.IsValid` _enemylock
    (:`Is Valid`
      (return (> (`KismetMathLibrary.VSize` (- (`KismetMathLibrary.Normal` (- (`self.K2_GetActorLocation` _enemylock) (`self.K2_GetActorLocation` (`self.Player`)))) (`SceneComponent.GetForwardVector` (`/Game/Proto/BP/BP_FPSPlayerCharacter.Camera` (`self.Player`))))) (`self.ThresholdGap`))))))

(fn `Fire`
  (bind _out (`self.Out`))
  (bind _player (`self.Player`))
  (bind _out_2 (`self.Out`))
  (`parent.Fire`)
  (if (`self.bIsLockToTarget`)
    (bind _outhit (`self.CastEnemyLock`))
    (cast `StaticMeshActor` (`.HitActor` (`GameplayStatics.BreakHitResult` _outhit)))
    (`self.OnReleaseShoot`)
    (else
      (bind _outhit_2 (`self.CastLine`))
      (bind _asbp_enemy_base (cast `/Game/Proto/BP/Enemies/BP_EnemyBase` (`.HitActor` (`GameplayStatics.BreakHitResult` _outhit_2)))
        (:`then`
          (set `self.EnemyLock` _asbp_enemy_base)
          (`self.PrepareScale`)
          (set `self.CanScale` false)
          (set `self.bIsLockToTarget` true)
          (`/Engine/EditorBlueprintResources/StandardMacros.IsValid` (`self.LazerBeam`)
            (:`Is Not Valid`
              (bind _returnvalue (`NiagaraFunctionLibrary.SpawnSystemAttached` "/Game/Proto/BP/Weapon/Lazer/LazerBeam_System.LazerBeam_System" _out "None" (`SceneComponent.K2_GetComponentLocation` _out) (struct) "KeepWorldPosition"))
              (bind _output_get (set `self.LazerBeam` _returnvalue))
              (`NiagaraComponent.SetVariableVec3` _output_get "User.BeamEnd" (`self.K2_GetActorLocation` (`self.EnemyLock`))))))
        (:`CastFailed`
          (`/Engine/EditorBlueprintResources/StandardMacros.IsValid` (`self.LazerBeam`)
            (:`Is Not Valid`
              (bind _returnvalue_2 (`NiagaraFunctionLibrary.SpawnSystemAttached` "/Game/Proto/BP/Weapon/Lazer/LazerBeam_System.LazerBeam_System" _out_2 "None" (`SceneComponent.K2_GetComponentLocation` _out_2) (struct) "KeepWorldPosition"))
              (bind _output_get_2 (set `self.LazerBeam` _returnvalue_2))
              (`NiagaraComponent.SetVariableVec3` _output_get_2 "User.BeamEnd" (+ (`self.K2_GetActorLocation` _player) (* (`SceneComponent.GetForwardVector` (`/Game/Proto/BP/BP_FPSPlayerCharacter.Camera` _player)) (`self.FireRange`)))))))))))

(fn `GetPlayerController`
  (bind _ascharacter (cast `Character` (`self.GetOwner`)))
  (bind _asbp_fpsplayer_character (cast `/Game/Proto/BP/BP_FPSPlayerCharacter` (`Controller.K2_GetPawn` (`Pawn.GetController` _ascharacter))))
  (set `self.Player` _asbp_fpsplayer_character))

(fn `OnReleaseShoot`
  (bind _lazerbeam (`self.LazerBeam`))
  (`parent.OnReleaseShoot`)
  (`/Engine/EditorBlueprintResources/StandardMacros.IsValid` _lazerbeam
    (:`Is Valid`
      (`ActorComponent.K2_DestroyComponent` _lazerbeam)
      (set `self.EnemyLock` null)
      (set `self.ScaleLevel` 0)
      (set `self.ScaleDamageTime` 2.0)
      (set `self.bIsLockToTarget` false)
      (set `self.CanScale` true))))

(fn `SetEnemyBeamEnd`
  (bind _lazerbeam (`self.LazerBeam`))
  (if (`self.bIsLockToTarget`)
    (`/Engine/EditorBlueprintResources/StandardMacros.IsValid` _lazerbeam
      (:`Is Valid`
        (`/Engine/EditorBlueprintResources/StandardMacros.IsValid` (`self.EnemyLock`)
          (:`Is Valid`
            (`NiagaraComponent.SetVariableVec3` _lazerbeam "User.BeamEnd" (`self.K2_GetActorLocation` (`self.EnemyLock`))))
          (:`Is Not Valid`
            (`self.OnReleaseShoot`)))))))

(fn `UserConstructionScript`
  (`parent.UserConstructionScript`))