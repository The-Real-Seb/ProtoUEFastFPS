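; Base weapon Blueprint that handles held-trigger automatic fire with a rate limit, leaving Fire as an empty function.
; OnShoot and OnReleaseShoot toggle the shooting flag, with OnShoot also attempting an immediate shot.
; Each shot sets a reload flag and starts a one-shot FireRate timer.
; When that timer ends, FinishReload clears the flag and re-triggers Shoot, which repeats while shooting stays active.
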(event `Prepare`
  (bind _returnvalue (`KismetSystemLibrary.K2_SetTimerDelegate` (delegate `FinishReload`) (`self.FireRate`))))

(event `FinishReload`
  (set `self.IsReload` false)
  (`KismetSystemLibrary.K2_SetTimerDelegate` (delegate `Shoot`) 0.001))

(event `Shoot`
  (if (`self.IsReload`)
    _
    (elif (`self.IsShooting`)
      (`self.Fire`)
      (set `self.IsReload` true)
      (`self.Prepare`)
      (else
        (`KismetSystemLibrary.K2_ClearAndInvalidateTimerHandle` (stale `Prepare` _returnvalue))))))

(fn `Fire`)

(fn `OnReleaseShoot`
  (set `self.IsShooting` false))

(fn `OnShoot`
  (set `self.IsShooting` true)
  (`self.Shoot`))

(fn `ShootLoop`
  (returns (IsShoot :type Boolean))
  (bind _returnvalue (`KismetSystemLibrary.K2_SetTimerDelegate` (delegate `Shoot`) (`self.FireRate`))))

(event `Shoot`
  (if (`self.IsShooting`)
    (return true)
    (else
      (`KismetSystemLibrary.K2_ClearAndInvalidateTimerHandle` (stale `ShootLoop` _returnvalue))
      (return false))))

(fn `UserConstructionScript`)