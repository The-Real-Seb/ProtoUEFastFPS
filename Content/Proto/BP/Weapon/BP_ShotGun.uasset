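; Shotgun weapon for the FPS player that overrides Fire to shoot a burst of hitscan pellets at enemies.
; Each pellet line-traces from the player's LineOriginPoint along its forward vector, with random per-axis Spread offsetting the endpoint at FireRange.
; Enemy hits scale Damage by the speed component's velocity-based bonus and pass it to the enemy's health component.
; Debug trace drawing and damage printing are left on.
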(fn `Fire`
  (bind _spread (`self.Spread`))
  (bind _spread_2 (`self.Spread`))
  (bind _spread_3 (`self.Spread`))
  (`parent.Fire`)
  (bind _ascharacter (cast `Character` (`self.GetOwner`)))
  (bind _asbp_fpsplayer_character (cast `/Game/Proto/BP/BP_FPSPlayerCharacter` (`Controller.K2_GetPawn` (`Pawn.GetController` _ascharacter))))
  (for _ (range 11)
    (bind _lineoriginpoint (`/Game/Proto/BP/BP_FPSPlayerCharacter.LineOriginPoint` _asbp_fpsplayer_character))
    (bind _returnvalue (`SceneComponent.K2_GetComponentLocation` _lineoriginpoint))
    (bind _outhit (`KismetSystemLibrary.LineTraceSingle` :`Start` _returnvalue :`End` (+ _returnvalue (* (`SceneComponent.GetForwardVector` _lineoriginpoint) (`self.FireRange`)) (`KismetMathLibrary.MakeVector` (`KismetMathLibrary.RandomFloatInRange` (* _spread_2 -1.0) _spread_2) (`KismetMathLibrary.RandomFloatInRange` (* _spread_3 -1.0) _spread_3) (`KismetMathLibrary.RandomFloatInRange` (* _spread -1.0) _spread))) :`TraceChannel` "TraceTypeQuery1" :`DrawDebugType` "ForDuration"))
    (bind _asbp_enemy_base (cast `/Game/Proto/BP/Enemies/BP_EnemyBase` (`.HitActor` (`GameplayStatics.BreakHitResult` _outhit))))
    (bind _asbp_fpsplayer_character_2 (cast `/Game/Proto/BP/BP_FPSPlayerCharacter` (`self.GetOwner`)))
    (bind _damagemultiply (`/Game/Proto/BP/BP_SpeedComponent.Get Bonus Damage` (`/Game/Proto/BP/BP_FPSPlayerCharacter.BP_SpeedComponent` _asbp_fpsplayer_character_2) (`self.GetVelocity` _asbp_fpsplayer_character_2)))
    (bind _returnvalue_2 (* _damagemultiply (`self.Damage`)))
    (`KismetSystemLibrary.PrintString` (`KismetStringLibrary.Conv_DoubleToString` _returnvalue_2) true true (struct :`G` 0.66 :`B` 1.0 :`A` 1.0) 1.0)
    (`/Game/Proto/BP/BP_HealthComponent.onHit` (`/Game/Proto/BP/Enemies/BP_EnemyBase.BP_HealthComponent` _asbp_enemy_base) _returnvalue_2)))

(fn `UserConstructionScript`
  (`parent.UserConstructionScript`))