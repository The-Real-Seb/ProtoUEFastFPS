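; Ranged enemy that chases the player and fires its weapon once within shooting distance.
; On BeginPlay it spawns the selected BP_Weapon, attaches it and configures targeting and fire rate; the weapon is destroyed with the enemy.
; Tick switches by distance between AIMoveTo pursuit, which clears the shooting state, and attack.
; Attack uses a DoOnce to halt movement, turns body and gun toward the player, and triggers OnShoot behind an IsShooting guard.
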(event `self.ReceiveDestroyed`
  (`self.K2_DestroyActor` (`self.CurrentWeapon`))
  (`KismetSystemLibrary.PrintString` "Destroy"))

(event `self.ReceiveBeginPlay`
  (set `self.ArrowLineOriginPoint` (`self.LineOriginPoint`))
  (bind _returnvalue (`|SpawnActorFromClass` (`.WeaponClass_7_AC8CD9AA4599F0B1A5232CA362FA3557` (break `/Game/Proto/BP/Weapon/SWeapon` (`self.SelectedWeapon`))) (`self.GetTransform`) "Undefined" "MultiplyWithRoot" self null))
  (`self.K2_AttachToComponent` _returnvalue (`self.LineOriginPoint`) "None" "KeepRelative" "KeepRelative" "KeepRelative" true)
  (bind _output_get (set `self.CurrentWeapon` _returnvalue))
  (bind _asbp_weapon (cast `/Game/Proto/BP/Weapon/BP_Weapon` _output_get))
  (set `/Game/Proto/BP/Weapon/BP_Weapon.IsEnemyTarget` false _asbp_weapon)
  (set `/Game/Proto/BP/Weapon/BP_Weapon.FireRate` (`self.TireRate`) _asbp_weapon)
  (set `self.isShooting` false))

(event `self.ReceiveTick`
  (params (DeltaSeconds :type "Float (single-precision)"))
  (bind _gun (`self.Gun`))
  (bind _returnvalue (+ (.pitch (`KismetMathLibrary.FindLookAtRotation` (`self.K2_GetActorLocation`) (`self.K2_GetActorLocation` (`GameplayStatics.GetPlayerCharacter` 0)))) 90.0))
  (if (> (`KismetMathLibrary.Vector_Distance` (`self.K2_GetActorLocation`) (`self.K2_GetActorLocation` (`GameplayStatics.GetPlayerCharacter` 0))) (`self.DistanceToShot`))
    (`|AIMoveTo` self (0.0 0.0 0.0) (`GameplayStatics.GetPlayerCharacter` 0) 50.0
      (:`then`
        (bind _asbp_weapon (cast `/Game/Proto/BP/Weapon/BP_Weapon` (`self.CurrentWeapon`)))
        (set `/Game/Proto/BP/Weapon/BP_Weapon.IsShooting` false _asbp_weapon)
        (set `self.isShooting` false)
        (goto _label :!via `Reset`)))
    (else
      (`|ExecutionSequence`
        (:`then_0`
          (`/Engine/EditorBlueprintResources/StandardMacros.DoOnce` false :!label _label
            (:`Completed`
              (`MovementComponent.StopMovementImmediately` (`self.CharacterMovement`)))))
        (:`then_1`
          (`self.K2_SetActorRotation` (`KismetMathLibrary.MakeRotator` 0.0 0.0 (.yaw (`KismetMathLibrary.FindLookAtRotation` (`self.K2_GetActorLocation`) (`self.K2_GetActorLocation` (`GameplayStatics.GetPlayerCharacter` 0))))))
          (`SceneComponent.K2_SetRelativeRotation` _gun (`KismetMathLibrary.MakeRotator` 0.0 _returnvalue) false false)
          (`SceneComponent.K2_SetWorldRotation` _gun (`KismetMathLibrary.MakeRotator` 0.0 _returnvalue (.yaw (`KismetMathLibrary.FindLookAtRotation` (`SceneComponent.K2_GetComponentLocation` _gun) (`self.K2_GetActorLocation` (`GameplayStatics.GetPlayerCharacter` 0))))) false false)
          (if (not (`self.isShooting`))
            (bind _asbp_weapon_2 (cast `/Game/Proto/BP/Weapon/BP_Weapon` (`self.CurrentWeapon`)))
            (`/Game/Proto/BP/Weapon/BP_Weapon.OnShoot` _asbp_weapon_2)
            (set `self.isShooting` true)))))))

(fn `UserConstructionScript`
  (`parent.UserConstructionScript`))