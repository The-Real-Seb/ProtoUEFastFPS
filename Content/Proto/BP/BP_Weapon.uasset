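; BP_Weapon is a prototype weapon that auto-fires BP_bullet actors at its own transform while Fire input is held.
; Pressing Fire shoots immediately, then each shot calls Prepare to set a one-shot ReloadTime timer back to Shoot, forming the repeat loop.
; Releasing only clears IsShooting, so the pending timer's next Shoot stops the loop.
; Debug prints report each outcome; OnShoot and Reload are empty stubs.
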(event `Prepare`
  (bind _returnvalue (`KismetSystemLibrary.K2_SetTimerDelegate` (delegate `Shoot`) (`self.ReloadTime`))))

(event `Shoot`
  (if (`self.IsShooting`)
    (`|SpawnActorFromClass` "/Game/Proto/BP/BP_bullet.BP_bullet_C" (`self.GetTransform`) "AlwaysSpawn" "MultiplyWithRoot" null null)
    (`KismetSystemLibrary.PrintString` "Shoot" true true (struct :`G` 0.66 :`B` 1.0 :`A` 1.0) -1.0)
    (`self.Prepare`)
    (else
      (`KismetSystemLibrary.PrintString` "ShootFailed" true true (struct :`G` 0.66 :`B` 1.0 :`A` 1.0) -1.0)
      (`KismetSystemLibrary.K2_ClearAndInvalidateTimerHandle` (stale `Prepare` _returnvalue)))))

(event `InputAction|Fire`
  (params (Key :type "Key Structure"))
  (:`Pressed`
    (set `self.IsShooting` true)
    (`self.Shoot`))
  (:`Released`
    (set `self.IsShooting` false)))

(fn `OnShoot`)

(fn `Reload`)

(fn `UserConstructionScript`)