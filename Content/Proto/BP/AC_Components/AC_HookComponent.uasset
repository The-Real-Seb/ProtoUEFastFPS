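; Actor component that gives the first-person player a grappling hook on the Hook input.
; Press line-traces from the character's origin point; a hit stores the grab point, switches to Flying, shows the cable and blocks move and dash.
; Tick pins the cable end and adds velocity impulses toward the point, bent by right-axis input for steering.
; Release restores Falling, movement and dash, then adds an impulse scaled from current velocity.
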(event `InputAction|Hook`
  (params (Key :type "Key Structure"))
  (bind _returnvalue (`GameplayStatics.GetPlayerCharacter` 0))
  ;[1 1 1] Grapping mechanique
  (:`Pressed`
    (bind _ascharacter (cast `Character` (`self.GetOwner`)))
    (bind _asbp_fpsplayer_character (cast `/Game/Proto/BP/BP_FPSPlayerCharacter` (`Controller.K2_GetPawn` (`Pawn.GetController` _ascharacter))))
    (bind _lineoriginpoint (`/Game/Proto/BP/BP_FPSPlayerCharacter.LineOriginPoint` _asbp_fpsplayer_character))
    (bind _returnvalue_2 (`SceneComponent.K2_GetComponentLocation` _lineoriginpoint))
    (bind (_outhit _returnvalue_3) (`KismetSystemLibrary.LineTraceSingle` :`Start` _returnvalue_2 :`End` (+ _returnvalue_2 (* (`SceneComponent.GetForwardVector` _lineoriginpoint) (`self.HookRange`))) :`TraceChannel` "TraceTypeQuery1" :`DrawDebugType` "ForDuration"))
    (if _returnvalue_3
      (set `self.GrabPoint` (`.ImpactPoint` (`GameplayStatics.BreakHitResult` _outhit)))
      (set `self.isGrapping` true)
      (bind _asbp_fpsplayer_character_2 (cast `/Game/Proto/BP/BP_FPSPlayerCharacter` _returnvalue))
      (`CharacterMovementComponent.SetMovementMode` (`Character.CharacterMovement` _returnvalue) "MOVE_Flying" 0)
      (`SceneComponent.SetVisibility` (`/Game/Proto/BP/BP_FPSPlayerCharacter.HookCable` _asbp_fpsplayer_character_2) true false)
      (set `/Game/Proto/BP/BP_FPSPlayerCharacter.RightAxisValue` 0.0 _asbp_fpsplayer_character_2)
      (set `/Game/Proto/BP/BP_FPSPlayerCharacter.CanMove` false _asbp_fpsplayer_character_2)
      (set `/Game/Proto/BP/BP_FPSPlayerCharacter.bCanDash` false _asbp_fpsplayer_character_2)))
  (:`Released`
    (set `self.isGrapping` false)
    (`CharacterMovementComponent.SetMovementMode` (`Character.CharacterMovement` (`GameplayStatics.GetPlayerCharacter` 0)) "MOVE_Falling" 0)
    (bind _asbp_fpsplayer_character_3 (cast `/Game/Proto/BP/BP_FPSPlayerCharacter` (`GameplayStatics.GetPlayerCharacter` 0)))
    (`SceneComponent.SetVisibility` (`/Game/Proto/BP/BP_FPSPlayerCharacter.HookCable` _asbp_fpsplayer_character_3) false false)
    (set `/Game/Proto/BP/BP_FPSPlayerCharacter.CanMove` true _asbp_fpsplayer_character_3)
    (set `/Game/Proto/BP/BP_FPSPlayerCharacter.bCanDash` true _asbp_fpsplayer_character_3)
    (bind _charactermovement (`Character.CharacterMovement` _asbp_fpsplayer_character_3))
    (`CharacterMovementComponent.AddImpulse` _charactermovement (* (`MovementComponent.Velocity` _charactermovement) (`self.ForceApplyMultiply`)) true)))

(event `self.ReceiveTick`
  (params (DeltaSeconds :type "Float (single-precision)"))
  (bind _returnvalue (`GameplayStatics.GetPlayerCharacter` 0))
  (if (`self.isGrapping`)
    (bind _asbp_fpsplayer_character (cast `/Game/Proto/BP/BP_FPSPlayerCharacter` _returnvalue))
    (set `CableComponent.EndLocation` (`KismetMathLibrary.InverseTransformLocation` (`Actor.GetTransform` _returnvalue) (`self.GrabPoint`)) (`/Game/Proto/BP/BP_FPSPlayerCharacter.HookCable` _asbp_fpsplayer_character))
    (bind _returnvalue_2 (* (`KismetMathLibrary.Normal` (+ (`KismetMathLibrary.GetDirectionUnitVector` (`Actor.K2_GetActorLocation` _asbp_fpsplayer_character) (`self.GrabPoint`)) (* (* (`Actor.GetActorRightVector` _asbp_fpsplayer_character) (`/Game/Proto/BP/BP_FPSPlayerCharacter.RightAxisValue` _asbp_fpsplayer_character)) 0.5))) (`self.HookForce`)))
    (`CharacterMovementComponent.AddImpulse` (`Character.CharacterMovement` _asbp_fpsplayer_character) _returnvalue_2 true)
    (set `self.ForceApply` _returnvalue_2)))