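; Actor component that gives the FPS player a kick, knocking back enemies on the Kick input.
; A debug-drawn sphere trace along the owner's forward vector finds a BP_EnemyBase, stops its movement and launches it along camera forward with fixed lift.
; The speed component's bonus damage, computed from player velocity, scales horizontal launch force.
; Each hit triggers brief global slow motion, which Tick lerps back toward normal speed.
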(event `InputAction|Kick`
  (params (Key :type "Key Structure"))
  (:`Pressed`
    (`self.Kick`)))

(event `SlowMotion`
  (`GameplayStatics.SetGlobalTimeDilation` 0.05)
  (`KismetSystemLibrary.Delay` 0.05)
  (set `self.bExitSlowMo` true))

(event `self.ReceiveTick`
  (params (DeltaSeconds :type "Float (single-precision)"))
  (bind _returnvalue (`KismetMathLibrary.Lerp` (`GameplayStatics.GetGlobalTimeDilation`) 1.0 (* (`self.LerpPower`) DeltaSeconds)))
  (if (`self.bExitSlowMo`)
    (`GameplayStatics.SetGlobalTimeDilation` _returnvalue)
    (`KismetSystemLibrary.PrintString` (`KismetStringLibrary.Conv_DoubleToString` _returnvalue))
    (if (> _returnvalue 0.95)
      (set `self.bExitSlowMo` false))))

(fn `Kick`
  (bind _rootcomponent (`Actor.RootComponent` (`self.GetOwner`)))
  (bind _returnvalue (`SceneComponent.K2_GetComponentLocation` _rootcomponent))
  (bind _outhit (`KismetSystemLibrary.SphereTraceSingle` :`Start` _returnvalue :`End` (+ _returnvalue (* (`KismetMathLibrary.GetForwardVector` (`SceneComponent.K2_GetComponentRotation` _rootcomponent)) (`self.kickDistance`))) :`Radius` 200.0 :`TraceChannel` "TraceTypeQuery1" :`DrawDebugType` "ForDuration"))
  (bind _asbp_enemy_base (cast `/Game/Proto/BP/Enemies/BP_EnemyBase` (`.HitActor` (`GameplayStatics.BreakHitResult` _outhit))))
  (bind _asbp_fpsplayer_character (cast `/Game/Proto/BP/BP_FPSPlayerCharacter` (`self.GetOwner`)))
  (`MovementComponent.StopMovementImmediately` (`Character.CharacterMovement` _asbp_enemy_base))
  (bind _damagemultiply (`/Game/Proto/BP/BP_SpeedComponent.Get Bonus Damage` (`/Game/Proto/BP/BP_FPSPlayerCharacter.BP_SpeedComponent` _asbp_fpsplayer_character) (`Actor.GetVelocity` _asbp_fpsplayer_character)))
  (`Character.LaunchCharacter` _asbp_enemy_base (`KismetMathLibrary.MakeVector` (.x (* _damagemultiply (* (`SceneComponent.GetForwardVector` (`/Game/Proto/BP/BP_FPSPlayerCharacter.Camera` _asbp_fpsplayer_character)) (`self.kickPower`)))) (.y (* _damagemultiply (* (`SceneComponent.GetForwardVector` (`/Game/Proto/BP/BP_FPSPlayerCharacter.Camera` _asbp_fpsplayer_character)) (`self.kickPower`)))) 500.0) true true)
  (`self.SlowMotion`)
  (`KismetSystemLibrary.PrintString` (`KismetStringLibrary.Conv_DoubleToString` _damagemultiply)))