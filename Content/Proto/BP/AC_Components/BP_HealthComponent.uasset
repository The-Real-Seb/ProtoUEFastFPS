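; Health component that applies incoming damage and restarts the current level when health runs out.
; OnHit subtracts damage from Health unless IsInvincible is set, then starts a brief invincibility window through a delayed custom event.
; A hit that would bring Health to zero or below reopens the level by name, even during the invincibility window.
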(event `invincible Delay`
  (set `self.isInvincible` true)
  (`KismetSystemLibrary.Delay` 0.2)
  (set `self.isInvincible` false))

(fn `onHit`
  (params (damage :type "Float (double-precision)"))
  (if (> (- (`self.health`) damage) 0.0)
    (if (not (`self.isInvincible`))
      ;[1 1 1] onHit has life
      (set `self.health` (- (`self.health`) damage))
      (`self.invincible Delay`))
    (else
      ;[1 1 1] onHit death
      (bind _returnvalue (`GameplayStatics.GetCurrentLevelName` true))
      (`GameplayStatics.OpenLevel` (`KismetStringLibrary.Conv_StringToName` _returnvalue)))))