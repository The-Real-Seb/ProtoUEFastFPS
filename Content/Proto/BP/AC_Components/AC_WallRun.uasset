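; AC_WallRun is a prototype component that detects walls while the FPS player character falls, to start a wall run.
; Each Tick, a debug-drawn sphere trace filters hits by normal slope, stores horizontal speed and starts a looping timer that overwrites velocity with WallRunDirection times that speed.
; The direction calculation from wall normal and velocity is never executed.
; StopWallRun clears the timer and records end time, but nothing here calls it.
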(event `self.ReceiveBeginPlay`
  ;[1 1 1] Init
  (bind _asbp_fpsplayer_character (cast `/Game/Proto/BP/BP_FPSPlayerCharacter` (`self.GetOwner`)))
  (set `self.Owner` _asbp_fpsplayer_character))

(event `StopWallRun`
  (set `self.WallRun` false)
  (`KismetSystemLibrary.K2_ClearAndInvalidateTimerHandle` (`self.WallRunTimerHandle`))
  (set `self.WallRunEndTime` (`KismetSystemLibrary.GetGameTimeInSeconds`)))

(event `RunWallRun`
  (set `MovementComponent.Velocity` (* (`self.WallRunDirection`) (`self.WallRunInitSpeed`)) (`Character.CharacterMovement` (`self.Owner`))))

(event `self.ReceiveTick`
  (params (DeltaSeconds :type "Float (single-precision)"))
  (bind _owner (`self.Owner`))
  (bind _returnvalue (`SceneComponent.K2_GetComponentLocation` (`Character.CapsuleComponent` _owner)))
  ;[1 1 1] WallRun
  (if (`NavMovementComponent.IsFalling` (`Character.CharacterMovement` _owner))
    (bind (_outhit _returnvalue_2) (`KismetSystemLibrary.SphereTraceSingleForObjects` :`Start` (+ _returnvalue (0.0 0.0 40.0)) :`End` (+ _returnvalue (0.0 0.0 -40.0)) :`Radius` 40.0 :`ObjectTypes` (`|MakeArray` "ObjectTypeQuery1" "ObjectTypeQuery2" :!type "EObjectTypeQuery Enum") :`DrawDebugType` "ForDuration"))
    (bind _z (.z (`.Normal` (`GameplayStatics.BreakHitResult` _outhit))))
    (if (and _returnvalue_2 (and (<= _z 0.71) (>= _z -0.28)))
      (if (not (`self.WallRun`))
        (set `self.WallRun` true)
        (set `self.WallRunInitSpeed` (`KismetMathLibrary.VSize` (`KismetMathLibrary.MakeVector` (.x (`MovementComponent.Velocity` (`Character.CharacterMovement` (`self.Owner`)))) (.y (`MovementComponent.Velocity` (`Character.CharacterMovement` (`self.Owner`)))))))
        (bind _returnvalue_3 (`KismetSystemLibrary.K2_SetTimerDelegate` (delegate `RunWallRun`) 0.01 true))
        (set `self.WallRunTimerHandle` _returnvalue_3)))))