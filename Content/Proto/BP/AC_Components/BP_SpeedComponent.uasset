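; Speed component that derives bonus damage and bonus bullet speed from a supplied velocity.
; Both functions use the X of the unit direction from velocity to zero, so only the reversed heading counts, not the magnitude.
; Damage bonus is that X scaled by BonusMultiply, made absolute, plus one.
; Bullet speed bonus is the signed X scaled by SpeedMultiply.
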(event `self.ReceiveBeginPlay`)

(fn `Get Bonus Damage`
  (params (velocity :type "Vector Structure"))
  (returns (damageMultiply :type "Float (double-precision)"))
  (bind _returnvalue_x (`KismetMathLibrary.BreakVector` (`KismetMathLibrary.GetDirectionUnitVector` velocity)))
  (return (+ (`KismetMathLibrary.Abs` (* (`self.bonusMultiply`) _returnvalue_x)) 1.0)))

(fn `GetBonusBulletSpeed`
  (params (velocity :type "Vector Structure"))
  (returns (bulletSpeed :type "Float (double-precision)"))
  (bind _returnvalue_x (`KismetMathLibrary.BreakVector` (`KismetMathLibrary.GetDirectionUnitVector` velocity)))
  (return (* (`self.speedMultiply`) _returnvalue_x)))